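; Player character Blueprint that handles movement, look, object interaction and closing an open widget.
; Enhanced Input drives yaw-relative movement and camera look, while Interact runs a debug-drawn visibility trace from the camera and sends an interface message to the hit actor.
; Q or Escape removes CurrentWidget, unpauses the game, hides the cursor and restores game-only input.
; The InteractionTrace function and construction script are empty.
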(event `Key|Q` :paused true
  (params (Key :type "Key Structure"))
  (bind _returnvalue (`GameplayStatics.GetPlayerController` 0))
  (:`Pressed`
    (`/Engine/EditorBlueprintResources/StandardMacros.IsValid` (`self.CurrentWidget`) :!label _label
      (:`Is Valid`
        (`Widget.RemoveFromParent` (`self.CurrentWidget`))
        (bind _asbp_player_character (cast `/Game/char/player/bp/BP_PlayerCharacter` (`GameplayStatics.GetPlayerCharacter` 0)))
        (set `/Game/char/player/bp/BP_PlayerCharacter.CurrentWidget` null _asbp_player_character)
        (`GameplayStatics.SetGamePaused` false)
        (set `PlayerController.bShowMouseCursor` false _returnvalue)
        (`WidgetBlueprintLibrary.SetInputMode_GameOnly` _returnvalue)))))

(event `Key|Escape` :paused true
  (params (Key :type "Key Structure"))
  (:`Pressed`
    (goto _label)))

(event `EnhancedInput|/Game/char/player/bp/IA_Interact`
  (params (ActionValue :type Boolean) (ElapsedSeconds :type "Float (double-precision)") (TriggeredSeconds :type "Float (double-precision)") (InputAction :type "InputAction Object Reference" :default "/Game/char/player/bp/IA_Interact.IA_Interact"))
  (bind _camera (`self.Camera`))
  (bind _returnvalue (`SceneComponent.K2_GetComponentLocation` _camera))
  (:`Triggered`
    (bind _outhit (`KismetSystemLibrary.LineTraceSingle` :`Start` _returnvalue :`End` (+ (* (`SceneComponent.GetForwardVector` _camera) 300.0) _returnvalue) :`TraceChannel` "TraceTypeQuery1" :`DrawDebugType` "ForDuration"))
    (message `/Game/interaction/BPI_Interaction.InteractWithObject` (`.HitActor` (`GameplayStatics.BreakHitResult` _outhit)))))

(event `EnhancedInput|/Game/char/player/bp/IA_MoveRight`
  (params (ActionValue :type "Float (double-precision)") (ElapsedSeconds :type "Float (double-precision)") (TriggeredSeconds :type "Float (double-precision)") (InputAction :type "InputAction Object Reference" :default "/Game/char/player/bp/IA_MoveRight.IA_MoveRight"))
  (bind (_returnvalue_roll _returnvalue_pitch _returnvalue_yaw) (`KismetMathLibrary.BreakRotator` (`self.GetControlRotation`)))
  (:`Triggered`
    (`self.AddMovementInput` (`KismetMathLibrary.GetRightVector` (`KismetMathLibrary.MakeRotator` 0.0 0.0 _returnvalue_yaw)) ActionValue)))

(event `EnhancedInput|/Game/char/player/bp/IA_MoveFwd`
  (params (ActionValue :type "Float (double-precision)") (ElapsedSeconds :type "Float (double-precision)") (TriggeredSeconds :type "Float (double-precision)") (InputAction :type "InputAction Object Reference" :default "/Game/char/player/bp/IA_MoveFwd.IA_MoveFwd"))
  (bind (_returnvalue_roll _returnvalue_pitch _returnvalue_yaw) (`KismetMathLibrary.BreakRotator` (`self.GetControlRotation`)))
  (:`Triggered`
    (`self.AddMovementInput` (`KismetMathLibrary.GetForwardVector` (`KismetMathLibrary.MakeRotator` 0.0 0.0 _returnvalue_yaw)) ActionValue)))

(event `EnhancedInput|/Game/char/player/bp/IA_LookX`
  (params (ActionValue :type "Float (double-precision)") (ElapsedSeconds :type "Float (double-precision)") (TriggeredSeconds :type "Float (double-precision)") (InputAction :type "InputAction Object Reference" :default "/Game/char/player/bp/IA_LookX.IA_LookX"))
  (:`Triggered`
    (`self.AddControllerYawInput` ActionValue)))

(event `EnhancedInput|/Game/char/player/bp/IA_LookY`
  (params (ActionValue :type "Float (double-precision)") (ElapsedSeconds :type "Float (double-precision)") (TriggeredSeconds :type "Float (double-precision)") (InputAction :type "InputAction Object Reference" :default "/Game/char/player/bp/IA_LookY.IA_LookY"))
  (:`Triggered`
    (`self.AddControllerPitchInput` ActionValue)))

(fn `Interaction Trace`)

(fn `UserConstructionScript`)