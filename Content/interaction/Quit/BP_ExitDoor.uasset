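; BP_ExitDoor is an interactable door that opens a quit confirmation prompt.
; On InteractwithObject it creates the W_QuitConfirmation widget, stores it as CurrentWidget on BP_PlayerCharacter and adds it to the viewport.
; It then pauses the game, switches input to Game and UI, and shows the mouse cursor.
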(event `/Game/interaction/BPI_Interaction.InteractWithObject`
  (bind _returnvalue (`GameplayStatics.GetPlayerController` 0))
  (bind _returnvalue_2 (`|CreateWidget` "/Game/interaction/Quit/W_QuitConfirmation.W_QuitConfirmation_C"))
  (bind _asbp_player_character (cast `/Game/char/player/bp/BP_PlayerCharacter` (`GameplayStatics.GetPlayerCharacter` 0)))
  (set `/Game/char/player/bp/BP_PlayerCharacter.CurrentWidget` _returnvalue_2 _asbp_player_character)
  (`UserWidget.AddToViewport` _returnvalue_2 0)
  (`GameplayStatics.SetGamePaused` true)
  (`WidgetBlueprintLibrary.SetInputMode_GameAndUIEx` _returnvalue null)
  (set `PlayerController.bShowMouseCursor` true _returnvalue))

(fn `UserConstructionScript`
  (`parent.UserConstructionScript`))